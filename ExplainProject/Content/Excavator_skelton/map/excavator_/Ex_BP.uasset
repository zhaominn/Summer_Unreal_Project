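; Excavator Blueprint with mouse-drag camera rotation and an early test for detecting the left lever under the cursor.
; Mouse buttons set click flags, and while the right is held, Enhanced Input mouse movement adds world pitch and yaw to the SpringArm.
; Tick runs a complex visibility trace under the cursor and prints a debug message when the physical material matches LeftLeverCollision.
; The left-click flag is not yet read here.
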(event Input|EnhancedActionEvents|EnhancedInputActionIA_MouseMove
  (params (ActionValue :type Vector%202D%20Structure) (ElapsedSeconds :type Float%20%28double-precision%29) (TriggeredSeconds :type Float%20%28double-precision%29) (InputAction :type Input%20Action%20Object%20Reference :default "/Game/Input/IA_MouseMove.IA_MouseMove"))
  ;[0.15 0.15 0.15 0.5] 카메라 회전
  (if (Variables|Default|Getclick_right?)
    (Transformation|AddWorldRotation (Variables|Default|GetSpringArm) (Math|Rotator|MakeRotator 0.0 (.y ActionValue) (.x ActionValue)) false false)))

(event EventTick
  (params (DeltaSeconds :type Float%20%28single-precision%29))
  (if (== (.physmat (.HitResult (Game|Player|GetHitResultUnderCursorbyChannel (Game|GetPlayerController 0) "TraceTypeQuery1" true))) (Variables|Default|Getleft_lever_collision))
    (Development|PrintString "Hello")))

(event Input|MouseEvents|LeftMouseButton
  (params (Key :type Key%20Structure :default "None"))
  ;[0.15 0.15 0.15 0.5] 좌측 마우스 클릭
  (:Pressed
    (Variables|Default|Setclick_left? true))
  (:Released
    (Variables|Default|Setclick_left? false)))

(event Input|MouseEvents|RightMouseButton
  (params (Key :type Key%20Structure :default "None"))
  ;[0.15 0.15 0.15 0.5] 우측 마우스 클릭
  (:Pressed
    (Variables|Default|Setclick_right? true))
  (:Released
    (Variables|Default|Setclick_right? false)))

(fn ConstructionScript)