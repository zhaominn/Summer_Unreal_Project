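; Interactive excavator actor that the player moves, spins and clicks to open an explanation level for the left lever.
; Enhanced Input drives world-space movement on keys and yaw rotation while the left mouse is held and dragged.
; Tick billboards the handle and two lever widget buttons toward the camera.
; Left clicks trace under the cursor by component, though only the left lever button opens a level.
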(event Input|EnhancedActionEvents|EnhancedInputActionIA_LeftMouse
  (params (ActionValue :type Boolean) (ElapsedSeconds :type Float%20%28double-precision%29) (TriggeredSeconds :type Float%20%28double-precision%29) (InputAction :type Input%20Action%20Object%20Reference :default "/Game/Input/IA_LeftMouse.IA_LeftMouse"))
  (:Triggered
    (CallFunction|StartExplain))
  (:Started
    (Variables|Default|Setclicking true))
  (:Completed
    (Variables|Default|Setclicking false)))

(event Input|EnhancedActionEvents|EnhancedInputActionIA_MouseMove
  (params (ActionValue :type Vector%202D%20Structure) (ElapsedSeconds :type Float%20%28double-precision%29) (TriggeredSeconds :type Float%20%28double-precision%29) (InputAction :type Input%20Action%20Object%20Reference :default "/Game/Input/IA_MouseMove.IA_MouseMove"))
  (if (Variables|Default|Getclicking)
    (Transformation|AddActorLocalRotation (Math|Rotator|MakeRotator 0.0 0.0 (* (.x ActionValue) -1.0)) false false)))

(event Input|EnhancedActionEvents|EnhancedInputActionIA_KeyMove
  (params (ActionValue :type Vector%202D%20Structure) (ElapsedSeconds :type Float%20%28double-precision%29) (TriggeredSeconds :type Float%20%28double-precision%29) (InputAction :type Input%20Action%20Object%20Reference :default "/Game/Input/IA_KeyMove.IA_KeyMove"))
  (Transformation|AddActorWorldOffset (Math|Vector|MakeVector (.x ActionValue) (.y ActionValue) 0.0)))

(event EventBeginPlay
  (Input|EnableInput (Game|GetPlayerController 0))
  (Utilities|Casting|CastToLeftLeverButton (UserInterface|GetUserWidgetObject (Variables|Default|GetLeftLeverExplainButton))))

(event Collision|EventActorBeginOverlap
  (params (OtherActor :type Actor%20Object%20Reference)))

(event EventTick
  (params (DeltaSeconds :type Float%20%28single-precision%29))
  (CallFunction|SetWidgetRotation))

(fn ConstructionScript)

(fn SetWidgetRotation
  (bind _handleexplainbutton (Variables|Default|GetHandleExplainButton))
  (bind _leftleverexplainbutton (Variables|Default|GetLeftLeverExplainButton))
  (bind _rightleverexplainbutton (Variables|Default|GetRightLeverExplainButton))
  (Transformation|SetWorldRotation _handleexplainbutton (Math|Rotator|FindLookatRotation (Transformation|GetWorldLocation _handleexplainbutton) (Camera|GetCameraLocation (Game|GetPlayerCameraManager 0))) false false)
  (Transformation|SetWorldRotation _leftleverexplainbutton (Math|Rotator|FindLookatRotation (Transformation|GetWorldLocation _leftleverexplainbutton) (Camera|GetCameraLocation (Game|GetPlayerCameraManager 0))) false false)
  (Transformation|SetWorldRotation _rightleverexplainbutton (Math|Rotator|FindLookatRotation (Transformation|GetWorldLocation _rightleverexplainbutton) (Camera|GetCameraLocation (Game|GetPlayerCameraManager 0))) false false))

(fn StartExplain
  (bind _returnvalue (Game|GetPlayerController 0))
  (bind (_hitresult _returnvalue_2) (Game|Player|GetHitResultUnderCursorbyChannel _returnvalue "TraceTypeQuery1" true))
  (if _returnvalue_2
    (if (== (Variables|Default|GetLeftLeverExplainButton) (.hitcomponent _hitresult))
      (Game|OpenLevel(byObjectReference) "/Game/cinematics/LS_LeftLever_Level.LS_LeftLever_Level"))))