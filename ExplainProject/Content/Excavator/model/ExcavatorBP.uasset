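; Excavator actor that the player moves and that carries in-world explain-button widgets for its handle and left and right levers.
; BeginPlay enables input from the first player controller, and IA_Move shifts the actor along world X and Y by the raw input value.
; Every Tick, SetWidgetRotation turns the three buttons to face the player camera.
; The left lever click handler is empty, and its widget cast on BeginPlay leads to no further logic.
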(event OnClicked(LeftLeverExplainButton)
  (params (TouchedComponent :type Primitive%20Component%20Object%20Reference) (ButtonPressed :type Key%20Structure :default "None")))

(event Input|EnhancedActionEvents|EnhancedInputActionIA_Move
  (params (ActionValue :type Vector%202D%20Structure) (ElapsedSeconds :type Float%20%28double-precision%29) (TriggeredSeconds :type Float%20%28double-precision%29) (InputAction :type Input%20Action%20Object%20Reference :default "/Game/Input/IA_Move.IA_Move"))
  (Transformation|AddActorWorldOffset (Math|Vector|MakeVector (.x ActionValue) (.y ActionValue) 0.0)))

(event EventBeginPlay
  (Input|EnableInput (Game|GetPlayerController 0))
  (Utilities|Casting|CastToLeftLeverButton (UserInterface|GetUserWidgetObject (Variables|Default|GetLeftLeverExplainButton))))

(event Collision|EventActorBeginOverlap
  (params (OtherActor :type Actor%20Object%20Reference)))

(event EventTick
  (params (DeltaSeconds :type Float%20%28single-precision%29))
  (CallFunction|SetWidgetRotation))

(fn ConstructionScript)

(fn SetWidgetRotation
  (bind _handleexplainbutton (Variables|Default|GetHandleExplainButton))
  (bind _leftleverexplainbutton (Variables|Default|GetLeftLeverExplainButton))
  (bind _rightleverexplainbutton (Variables|Default|GetRightLeverExplainButton))
  (Transformation|SetWorldRotation _handleexplainbutton (Math|Rotator|FindLookatRotation (Transformation|GetWorldLocation _handleexplainbutton) (Camera|GetCameraLocation (Game|GetPlayerCameraManager 0))) false false)
  (Transformation|SetWorldRotation _leftleverexplainbutton (Math|Rotator|FindLookatRotation (Transformation|GetWorldLocation _leftleverexplainbutton) (Camera|GetCameraLocation (Game|GetPlayerCameraManager 0))) false false)
  (Transformation|SetWorldRotation _rightleverexplainbutton (Math|Rotator|FindLookatRotation (Transformation|GetWorldLocation _rightleverexplainbutton) (Camera|GetCameraLocation (Game|GetPlayerCameraManager 0))) false false))