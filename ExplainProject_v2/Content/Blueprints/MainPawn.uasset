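; MainPawn is the player pawn for an excavator tutorial: it shows an explanation widget, exposes a text update for it, and sets the view to the Excavator.
; Mouse clicks trace under the cursor and send MouseClickMessage to the hit actor, while movement and arrow keys only print placeholder text.
; MakeCameraLookAt aims a child-actor TargetPoint, blends to it, then swaps it with a second one, so successive camera moves alternate targets.
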(event Input|EnhancedActionEvents|EnhancedInputActionIA_Up
  (params (ActionValue :type Boolean) (ElapsedSeconds :type Float%20%28double-precision%29) (TriggeredSeconds :type Float%20%28double-precision%29) (InputAction :type Input%20Action%20Object%20Reference :default "/Game/Input/Right_Lever/IA_Up.IA_Up"))
  ;[0.15 0.15 0.15 0.5] (임시)Key Input
  (Development|PrintText "Up"))

(event Input|EnhancedActionEvents|EnhancedInputActionIA_Down
  (params (ActionValue :type Boolean) (ElapsedSeconds :type Float%20%28double-precision%29) (TriggeredSeconds :type Float%20%28double-precision%29) (InputAction :type Input%20Action%20Object%20Reference :default "/Game/Input/Right_Lever/IA_Down.IA_Down"))
  ;[0.15 0.15 0.15 0.5] (임시)Key Input
  (Development|PrintText "Down"))

(event Input|EnhancedActionEvents|EnhancedInputActionIA_A
  (params (ActionValue :type Boolean) (ElapsedSeconds :type Float%20%28double-precision%29) (TriggeredSeconds :type Float%20%28double-precision%29) (InputAction :type Input%20Action%20Object%20Reference :default "/Game/Input/Left_Lever/IA_A.IA_A"))
  ;[0.15 0.15 0.15 0.5] (임시)Key Input
  (Development|PrintText "A"))

(event Input|EnhancedActionEvents|EnhancedInputActionIA_S
  (params (ActionValue :type Boolean) (ElapsedSeconds :type Float%20%28double-precision%29) (TriggeredSeconds :type Float%20%28double-precision%29) (InputAction :type Input%20Action%20Object%20Reference :default "/Game/Input/Left_Lever/IA_S.IA_S"))
  ;[0.15 0.15 0.15 0.5] (임시)Key Input
  (Development|PrintText "S"))

(event Input|EnhancedActionEvents|EnhancedInputActionIA_D
  (params (ActionValue :type Boolean) (ElapsedSeconds :type Float%20%28double-precision%29) (TriggeredSeconds :type Float%20%28double-precision%29) (InputAction :type Input%20Action%20Object%20Reference :default "/Game/Input/Left_Lever/IA_D.IA_D"))
  ;[0.15 0.15 0.15 0.5] (임시)Key Input
  (Development|PrintText "D"))

(event Input|EnhancedActionEvents|EnhancedInputActionIA_Left
  (params (ActionValue :type Boolean) (ElapsedSeconds :type Float%20%28double-precision%29) (TriggeredSeconds :type Float%20%28double-precision%29) (InputAction :type Input%20Action%20Object%20Reference :default "/Game/Input/Right_Lever/IA_Left.IA_Left"))
  ;[0.15 0.15 0.15 0.5] (임시)Key Input
  (Development|PrintText "Left"))

(event Input|EnhancedActionEvents|EnhancedInputActionIA_Right
  (params (ActionValue :type Boolean) (ElapsedSeconds :type Float%20%28double-precision%29) (TriggeredSeconds :type Float%20%28double-precision%29) (InputAction :type Input%20Action%20Object%20Reference :default "/Game/Input/Right_Lever/IA_Right.IA_Right"))
  ;[0.15 0.15 0.15 0.5] (임시)Key Input
  (Development|PrintText "Right"))

(event Input|EnhancedActionEvents|EnhancedInputActionIA_MouseClick
  (params (ActionValue :type Boolean) (ElapsedSeconds :type Float%20%28double-precision%29) (TriggeredSeconds :type Float%20%28double-precision%29) (InputAction :type Input%20Action%20Object%20Reference :default "/Game/Input/IA_MouseClick.IA_MouseClick"))
  (Class|ComponentInterface|MouseClick(Message) (.HitActor (Collision|BreakHitResult (.HitResult (Game|Player|GetHitResultUnderCursorbyChannel (Game|GetPlayerController 0) "TraceTypeQuery1" true))))))

(event Input|EnhancedActionEvents|EnhancedInputActionIA_W
  (params (ActionValue :type Boolean) (ElapsedSeconds :type Float%20%28double-precision%29) (TriggeredSeconds :type Float%20%28double-precision%29) (InputAction :type Input%20Action%20Object%20Reference :default "/Game/Input/Left_Lever/IA_W.IA_W"))
  ;[0.15 0.15 0.15 0.5] (임시)Key Input
  (Development|PrintText "W"))

(event EventBeginPlay
  ;[0.15 0.15 0.15 0.5] 튜토리얼 설명 위젯
  (bind _returnvalue (UserInterface|CreateWidget "/Game/UI/Explain/Explain_Widget.Explain_Widget_C"))
  (UserInterface|Viewport|AddtoViewport _returnvalue 0)
  (Variables|Default|SetWidget_1 _returnvalue)
  (bind _returnvalue_2 (Actor|GetActorOfClass "/Game/Model/Excavator/Excavator.Excavator_C"))
  (bind _output_get (Variables|Default|SetExcavatorRef _returnvalue_2))
  (Game|Player|SetViewTargetwithBlend (Game|GetPlayerController 0) _output_get 0.0 "VTBlend_Linear" 0.0 false))

(event Collision|EventActorBeginOverlap
  (params (OtherActor :type Actor%20Object%20Reference)))

(event EventTick
  (params (DeltaSeconds :type Float%20%28single-precision%29)))

(fn ConstructionScript
  (bind _astarget_point (Utilities|Casting|CastToTargetPoint (Variables|/Script/Engine.ChildActorComponent|GetChildActor (Variables|Default|GetCameraLocator%20A))))
  (Variables|Default|SetView%20Target%20A _astarget_point)
  (bind _astarget_point_2 (Utilities|Casting|CastToTargetPoint (Variables|/Script/Engine.ChildActorComponent|GetChildActor (Variables|Default|GetCameraLocator%20B))))
  (Variables|Default|SetView%20Target%20B _astarget_point_2))

(fn MakeCameraLookat
  (params (From :type Vector) (To :type Vector))
  (LocalVariables|SetView%20Targert%20Location From)
  (LocalVariables|SetView%20Target%20Rotation (Math|Rotator|FindLookatRotation From To))
  (Transformation|SetActorLocationAndRotation (Variables|Default|GetView%20Target%20A) (LocalVariables|GetView%20Targert%20Location) (LocalVariables|GetView%20Target%20Rotation))
  (Game|Player|SetViewTargetwithBlend (Game|GetPlayerController 0) (Variables|Default|GetView%20Target%20A) 0.5 "VTBlend_Linear" 0.0 false)
  (Variables|Default|SetTemp%20Target (Variables|Default|GetView%20Target%20A))
  (Variables|Default|SetView%20Target%20A (Variables|Default|GetView%20Target%20B))
  (Variables|Default|SetView%20Target%20B (Variables|Default|GetTemp%20Target)))

(fn UpdateExplain
  (params (text :type Text))
  (Default|UpdateExplainText (Variables|Default|GetWidget_1) text))