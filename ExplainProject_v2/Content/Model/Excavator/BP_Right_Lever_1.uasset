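; Excavator right lever actor that animates the lever and the matching arm and bucket motion for demonstrations and tutorials.
; Four directional functions play a lever sequence and its BP_Arm_Basket counterpart, found through the parent Excavator or Excavator_Simulation.
; ExplainComponent demonstrates each direction on timed delays with Korean text and UI highlights, then finishes its behavior tree task.
; Tutorial events show key prompts on MainPawn, and finished lever sequences fire OnWorkFinished.
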(event Custom|CustomEvent
  ;[0.15 0.15 0.15 0.5] 이벤트 바인딩
  (Default|CallOnWorkFinished))

(event Custom|initLeverUI
  (params (Lever%20UI :type Lever%20UI%20Object%20Reference))
  ;[0.15 0.15 0.15 0.5] 레버 ui 가져옴
  (Variables|Default|SetRight%20Lever%20UI%20Widget Lever%20UI))

(event EventExplainComponent
  (params (BT :type Object%20Object%20Reference))
  (bind _right_lever_ui_widget (Variables|Default|GetRight%20Lever%20UI%20Widget))
  ;[0.15 0.15 0.15 0.5] Explain Component
  (Development|SetHiddeninGame (Variables|Default|GetHand%20Actor) false false)
  (CallFunction|ExplainBack)
  (Utilities|FlowControl|Delay 2.0)
  (Default|DefaultBtnColor _right_lever_ui_widget)
  (CallFunction|ExplainFront)
  (Utilities|FlowControl|Delay 2.0)
  (Default|DefaultBtnColor _right_lever_ui_widget)
  (CallFunction|ExplainLeft)
  (Utilities|FlowControl|Delay 2.0)
  (Default|DefaultBtnColor _right_lever_ui_widget)
  (CallFunction|ExplainRight)
  (Utilities|FlowControl|Delay 2.0)
  (Default|DefaultBtnColor _right_lever_ui_widget)
  (bind _asexplain_right_lever_bttask (Utilities|Casting|CastToExplain_RightLever_BTtask BT))
  (AI|BehaviorTree|FinishExecute _asexplain_right_lever_bttask true)
  (Development|SetHiddeninGame (Variables|Default|GetHand%20Actor) true false))

(event Collision|EventActorBeginOverlap
  (params (OtherActor :type Actor%20Object%20Reference))
  (|CallParentFunction OtherActor))

(event EventBeginPlay
  ;[0.15 0.15 0.15 0.5] 이벤트 바인딩
  (Input|EnableInput 0)
  (|CallParentFunction)
  (EventDispatchers|BindEventtoOnFinished (Variables|/Script/ActorSequence.ActorSequenceComponent|GetSequencePlayer (Variables|Default|GetLeftSequence)) (delegate Custom|CustomEvent))
  (EventDispatchers|BindEventtoOnFinished (Variables|/Script/ActorSequence.ActorSequenceComponent|GetSequencePlayer (Variables|Default|GetRightSequence)) (delegate Custom|CustomEvent))
  (EventDispatchers|BindEventtoOnFinished (Variables|/Script/ActorSequence.ActorSequenceComponent|GetSequencePlayer (Variables|Default|GetBackSequence)) (delegate Custom|CustomEvent))
  (EventDispatchers|BindEventtoOnFinished (Variables|/Script/ActorSequence.ActorSequenceComponent|GetSequencePlayer (Variables|Default|GetFrontSequence)) (delegate Custom|CustomEvent)))

(event EventTick
  (params (DeltaSeconds :type Float%20%28single-precision%29))
  (|CallParentFunction DeltaSeconds))

(event EventTutorialBack
  ;[0.15 0.15 0.15 0.5] Tutorial Right Lever
  (bind _asmain_pawn (Utilities|Casting|CastToMainPawn (Game|Player|GetPlayerPawn 0)))
  (Default|UpdateExplain _asmain_pawn "아래 방향키를 눌러 우측 레버를 아래쪽으로 움직이세요."))

(event EventTutorialFront
  ;[0.15 0.15 0.15 0.5] Tutorial Right Lever
  (bind _asmain_pawn (Utilities|Casting|CastToMainPawn (Game|Player|GetPlayerPawn 0)))
  (Default|UpdateExplain _asmain_pawn "위 방향키를 눌러 우측 레버를 앞으로 움직이세요."))

(event EventTutorialLeft
  ;[0.15 0.15 0.15 0.5] Tutorial Right Lever
  (bind _asmain_pawn (Utilities|Casting|CastToMainPawn (Game|Player|GetPlayerPawn 0)))
  (Default|UpdateExplain _asmain_pawn "좌측 방향키를 눌러 우측 레버를 왼쪽으로 움직이세요."))

(event EventTutorialRight
  ;[0.15 0.15 0.15 0.5] Tutorial Right Lever
  (bind _asmain_pawn (Utilities|Casting|CastToMainPawn (Game|Player|GetPlayerPawn 0)))
  (Default|UpdateExplain _asmain_pawn "우측 방향키를 눌러 우측 레버를 오른쪽으로 움직이세요."))

(fn ConstructionScript)

(fn PlayBackSequence
  (bind _returnvalue (Actor|GetParentActor))
  (Class|ActorSequenceComponent|PlaySequence (Variables|Default|GetBackSequence))
  (bind _asexcavator (Utilities|Casting|CastToExcavator _returnvalue)
    (:then
      (bind _asbp_arm_basket (Utilities|Casting|CastToBP_Arm_Basket (Variables|/Script/Engine.ChildActorComponent|GetChildActor (Variables|/Game/Model/Excavator/Excavator.Excavator_C|GetBP_Arm_Basket _asexcavator))))
      (Default|PlayArmBackSequence _asbp_arm_basket))
    (:CastFailed
      (bind _asexcavator_simulation (Utilities|Casting|CastToExcavator_Simulation _returnvalue))
      (bind _asbp_arm_basket_2 (Utilities|Casting|CastToBP_Arm_Basket (Variables|/Script/Engine.ChildActorComponent|GetChildActor (Variables|/Game/Model/Excavator/Excavator_Simulation.Excavator_Simulation_C|GetBP_Arm_Basket _asexcavator_simulation))))
      (Default|PlayArmBackSequence _asbp_arm_basket_2))))

(fn PlayFrontSequence
  (bind _returnvalue (Actor|GetParentActor))
  (Class|ActorSequenceComponent|PlaySequence (Variables|Default|GetFrontSequence))
  (bind _asexcavator (Utilities|Casting|CastToExcavator _returnvalue)
    (:then
      (bind _asbp_arm_basket (Utilities|Casting|CastToBP_Arm_Basket (Variables|/Script/Engine.ChildActorComponent|GetChildActor (Variables|/Game/Model/Excavator/Excavator.Excavator_C|GetBP_Arm_Basket _asexcavator))))
      (Default|PlayArmFrontSequence _asbp_arm_basket))
    (:CastFailed
      (bind _asexcavator_simulation (Utilities|Casting|CastToExcavator_Simulation _returnvalue))
      (bind _asbp_arm_basket_2 (Utilities|Casting|CastToBP_Arm_Basket (Variables|/Script/Engine.ChildActorComponent|GetChildActor (Variables|/Game/Model/Excavator/Excavator_Simulation.Excavator_Simulation_C|GetBP_Arm_Basket _asexcavator_simulation))))
      (Default|PlayArmFrontSequence _asbp_arm_basket_2))))

(fn PlayLeftSequence
  (bind _returnvalue (Actor|GetParentActor))
  (Class|ActorSequenceComponent|PlaySequence (Variables|Default|GetLeftSequence))
  (bind _asexcavator (Utilities|Casting|CastToExcavator _returnvalue)
    (:then
      (bind _asbp_arm_basket (Utilities|Casting|CastToBP_Arm_Basket (Variables|/Script/Engine.ChildActorComponent|GetChildActor (Variables|/Game/Model/Excavator/Excavator.Excavator_C|GetBP_Arm_Basket _asexcavator))))
      (Default|PlayBasketFrontSequence _asbp_arm_basket))
    (:CastFailed
      (bind _asexcavator_simulation (Utilities|Casting|CastToExcavator_Simulation _returnvalue))
      (bind _asbp_arm_basket_2 (Utilities|Casting|CastToBP_Arm_Basket (Variables|/Script/Engine.ChildActorComponent|GetChildActor (Variables|/Game/Model/Excavator/Excavator_Simulation.Excavator_Simulation_C|GetBP_Arm_Basket _asexcavator_simulation))))
      (Default|PlayBasketFrontSequence _asbp_arm_basket_2))))

(fn PlayRightSequence
  (bind _returnvalue (Actor|GetParentActor))
  (Class|ActorSequenceComponent|PlaySequence (Variables|Default|GetRightSequence))
  (bind _asexcavator (Utilities|Casting|CastToExcavator _returnvalue)
    (:then
      (bind _asbp_arm_basket (Utilities|Casting|CastToBP_Arm_Basket (Variables|/Script/Engine.ChildActorComponent|GetChildActor (Variables|/Game/Model/Excavator/Excavator.Excavator_C|GetBP_Arm_Basket _asexcavator))))
      (Default|PlayBasketBackSequence _asbp_arm_basket))
    (:CastFailed
      (bind _asexcavator_simulation (Utilities|Casting|CastToExcavator_Simulation _returnvalue))
      (bind _asbp_arm_basket_2 (Utilities|Casting|CastToBP_Arm_Basket (Variables|/Script/Engine.ChildActorComponent|GetChildActor (Variables|/Game/Model/Excavator/Excavator_Simulation.Excavator_Simulation_C|GetBP_Arm_Basket _asexcavator_simulation))))
      (Default|PlayBasketBackSequence _asbp_arm_basket_2))))

(fn ExplainBack
  (bind _asmain_pawn (Utilities|Casting|CastToMainPawn (Game|Player|GetPlayerPawn 0)))
  (Default|UpdateExplain _asmain_pawn "아래 방향키를 눌러 우측 레버를 뒤로 움직이면 버킷이 위로 올라갑니다.")
  (Default|ChangeBtnColorRBack (Variables|Default|GetRight%20Lever%20UI%20Widget))
  (CallFunction|PlayBackSequence))

(fn ExplainFront
  (bind _asmain_pawn (Utilities|Casting|CastToMainPawn (Game|Player|GetPlayerPawn 0)))
  (Default|UpdateExplain _asmain_pawn "위 방향키를 눌러 우측 레버를 앞으로 움직이면 버킷이 아래로 내려갑니다.")
  (Default|ChangeBtnColorRFront (Variables|Default|GetRight%20Lever%20UI%20Widget))
  (CallFunction|PlayFrontSequence))

(fn ExplainLeft
  (bind _asmain_pawn (Utilities|Casting|CastToMainPawn (Game|Player|GetPlayerPawn 0)))
  (Default|UpdateExplain _asmain_pawn "좌측 방향키를 눌러 우측 레버를 왼쪽으로 움직이면 버킷이 바깥쪽으로 회전합니다.")
  (Default|ChangeBtnColorRLeft (Variables|Default|GetRight%20Lever%20UI%20Widget))
  (CallFunction|PlayLeftSequence))

(fn ExplainRight
  (bind _asmain_pawn (Utilities|Casting|CastToMainPawn (Game|Player|GetPlayerPawn 0)))
  (Default|UpdateExplain _asmain_pawn "우측 방향키를 눌러 우측 레버를 오른쪽으로 움직이면 버킷이 안쪽으로 회전합니다.")
  (Default|ChangeBtnColorRRight (Variables|Default|GetRight%20Lever%20UI%20Widget))
  (CallFunction|PlayRightSequence))