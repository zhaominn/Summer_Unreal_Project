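; Excavator left lever actor that demonstrates and prompts the drive and rotate controls in the tutorial.
; Each direction plays a lever sequence alongside the matching move or rotate sequence on the parent Excavator, and finished lever sequences call OnWorkFinished.
; ExplainComponent steps through all four directions on timed delays, updating MainPawn text and highlighting back/front UI buttons, then completes its Behavior Tree task.
; Tutorial events show one drag instruction and play that direction.
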(event Custom|CustomEvent
  ;[0.15 0.15 0.15 0.5] 이벤트 바인딩
  (Default|CallOnWorkFinished))

(event Custom|initLeverUI
  (params (Lever%20UI :type Lever%20UI%20Object%20Reference))
  ;[0.15 0.15 0.15 0.5] 레버 ui 가져옴
  (Variables|Default|Setlever_ui_widget Lever%20UI))

(event Collision|EventActorBeginOverlap
  (params (OtherActor :type Actor%20Object%20Reference))
  (|CallParentFunction OtherActor))

(event EventTick
  (params (DeltaSeconds :type Float%20%28single-precision%29))
  (|CallParentFunction DeltaSeconds))

(event EventBeginPlay
  ;[0.15 0.15 0.15 0.5] 이벤트 바인딩
  (|CallParentFunction)
  (EventDispatchers|BindEventtoOnFinished (Variables|/Script/ActorSequence.ActorSequenceComponent|GetSequencePlayer (Variables|Default|GetLeftSequence)) (delegate Custom|CustomEvent))
  (EventDispatchers|BindEventtoOnFinished (Variables|/Script/ActorSequence.ActorSequenceComponent|GetSequencePlayer (Variables|Default|GetRightSequence)) (delegate Custom|CustomEvent))
  (EventDispatchers|BindEventtoOnFinished (Variables|/Script/ActorSequence.ActorSequenceComponent|GetSequencePlayer (Variables|Default|GetBackSequence)) (delegate Custom|CustomEvent))
  (EventDispatchers|BindEventtoOnFinished (Variables|/Script/ActorSequence.ActorSequenceComponent|GetSequencePlayer (Variables|Default|GetFrontSequence)) (delegate Custom|CustomEvent)))

(event EventExplainComponent
  (params (BT :type Object%20Object%20Reference))
  (bind _lever_ui_widget (Variables|Default|Getlever_ui_widget))
  (bind _lever_ui_widget_2 (Variables|Default|Getlever_ui_widget))
  ;[0.15 0.15 0.15 0.5] Explain Component
  (bind _asmain_pawn (Utilities|Casting|CastToMainPawn (Game|Player|GetPlayerPawn 0)))
  (Default|UpdateExplain _asmain_pawn "좌측 레버를 뒤로 드래그 하면 포크레인이 후진합니다.")
  (Default|ChangeBtnColorLBack _lever_ui_widget_2)
  (CallFunction|PlayBackSequence)
  (Utilities|FlowControl|Delay 2.0)
  (Default|DefaultBtnColor _lever_ui_widget_2)
  (Default|ChangeBtnColorLFront _lever_ui_widget)
  (Default|UpdateExplain _asmain_pawn "좌측 레버를 앞으로 드래그 하면 포크레인이 전진합니다.")
  (CallFunction|PlayFrontSequence)
  (Utilities|FlowControl|Delay 2.0)
  (Default|DefaultBtnColor _lever_ui_widget)
  (Default|UpdateExplain _asmain_pawn "좌측 레버를 오른쪽으로 드래그 하면 포크레인이 왼쪽으로 회전합니다.")
  (CallFunction|PlayLeftSequence)
  (Utilities|FlowControl|Delay 2.0)
  (Default|UpdateExplain _asmain_pawn "좌측 레버를 왼쪽으로 드래그 하면 포크레인이 오른쪽으로 회전합니다.")
  (CallFunction|PlayRightSequence)
  (Utilities|FlowControl|Delay 2.0)
  (bind _asexplain_left_lever_bttask (Utilities|Casting|CastToExplain_LeftLever_BTtask BT))
  (AI|BehaviorTree|FinishExecute _asexplain_left_lever_bttask true))

(event EventTutorialFront
  (bind _asmain_pawn (Utilities|Casting|CastToMainPawn (Game|Player|GetPlayerPawn 0)))
  (Default|UpdateExplain _asmain_pawn "좌측 레버를 앞으로 드래그 하세요.")
  (CallFunction|PlayFrontSequence))

(event EventTutorialBack
  (bind _asmain_pawn (Utilities|Casting|CastToMainPawn (Game|Player|GetPlayerPawn 0)))
  (Default|UpdateExplain _asmain_pawn "좌측 레버를 뒤로 드래그 하세요.")
  (CallFunction|PlayBackSequence))

(event EventTutorialLeft
  (bind _asmain_pawn (Utilities|Casting|CastToMainPawn (Game|Player|GetPlayerPawn 0)))
  (Default|UpdateExplain _asmain_pawn "좌측 레버를 왼쪽으로 드래그 하세요.")
  (CallFunction|PlayLeftSequence))

(event EventTutorialRight
  (bind _asmain_pawn (Utilities|Casting|CastToMainPawn (Game|Player|GetPlayerPawn 0)))
  (Default|UpdateExplain _asmain_pawn "좌측 레버를 오른쪽으로 드래그 하세요.")
  (CallFunction|PlayRightSequence))

(fn ConstructionScript)

(fn PlayBackSequence
  (Class|ActorSequenceComponent|PlaySequence (Variables|Default|GetBackSequence))
  (bind _asexcavator (Utilities|Casting|CastToExcavator (Actor|GetParentActor)))
  (Class|ActorSequenceComponent|PlaySequence (Variables|/Game/Model/Excavator/Excavator.Excavator_C|GetMoveBack _asexcavator)))

(fn PlayFrontSequence
  (Class|ActorSequenceComponent|PlaySequence (Variables|Default|GetFrontSequence))
  (bind _asexcavator (Utilities|Casting|CastToExcavator (Actor|GetParentActor)))
  (Class|ActorSequenceComponent|PlaySequence (Variables|/Game/Model/Excavator/Excavator.Excavator_C|GetMoveFront _asexcavator)))

(fn PlayLeftSequence
  (Class|ActorSequenceComponent|PlaySequence (Variables|Default|GetLeftSequence))
  (bind _asexcavator (Utilities|Casting|CastToExcavator (Actor|GetParentActor)))
  (Class|ActorSequenceComponent|PlaySequence (Variables|/Game/Model/Excavator/Excavator.Excavator_C|GetRotateLeft _asexcavator)))

(fn PlayRightSequence
  (Class|ActorSequenceComponent|PlaySequence (Variables|Default|GetRightSequence))
  (bind _asexcavator (Utilities|Casting|CastToExcavator (Actor|GetParentActor)))
  (Class|ActorSequenceComponent|PlaySequence (Variables|/Game/Model/Excavator/Excavator.Excavator_C|GetRotateRight _asexcavator)))