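; BP_Right_Lever is the excavator's right lever Blueprint, with an event that demonstrates the lever's four directions.
; ExplainRightLever plays the back, front, left and right sequences in that order, using fixed delays to space them rather than waiting for each to finish.
; The Blueprint has no other active logic, so the demonstration runs only when that event is called.
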(event EventBeginPlay)

(event Collision|EventActorBeginOverlap
  (params (OtherActor :type Actor%20Object%20Reference)))

(event EventTick
  (params (DeltaSeconds :type Float%20%28single-precision%29)))

(event EventExplainRightLever
  (Class|ActorSequenceComponent|PlaySequence (Variables|Default|GetBackSequence))
  (Utilities|FlowControl|Delay 2.0)
  (Class|ActorSequenceComponent|PlaySequence (Variables|Default|GetFrontSequence))
  (Utilities|FlowControl|Delay 2.0)
  (Class|ActorSequenceComponent|PlaySequence (Variables|Default|GetLeftSequence))
  (Utilities|FlowControl|Delay 2.0)
  (Class|ActorSequenceComponent|PlaySequence (Variables|Default|GetRightSequence))
  (Utilities|FlowControl|Delay 2.0))

(fn ConstructionScript)